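; Breakable door actor that loses health each time DoorTakeDamage is called and is destroyed when it runs out.
; Each call subtracts a fixed amount from CurrentHealth, then either refreshes the health bar or calls DoorDie.
; The bar is a widget component whose WB_AIHealthBar receives the current-to-max health ratio.
; The event graph is empty, so nothing in this Blueprint triggers the damage itself.
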(fn `DoorDie`
  (`self.K2_DestroyActor`))

(fn `DoorTakeDamage`
  (set `self.CurrentHealth` (- (`self.CurrentHealth`) 30))
  (if (> (`self.CurrentHealth`) 0)
    (`self.DoorUpdateHealthbar`)
    (else
      (`self.DoorDie`))))

(fn `DoorUpdateHealthbar`
  (bind _aswb_aihealth_bar (cast `/Game/SamanthaAssets/AI/WB_AIHealthBar` (`WidgetComponent.GetUserWidgetObject` (`self.Healthbar`))))
  (set `/Game/SamanthaAssets/AI/WB_AIHealthBar.HealthPercentage` (/ (`KismetMathLibrary.Conv_IntToDouble` (`self.CurrentHealth`)) (`KismetMathLibrary.Conv_IntToDouble` (`self.MaxHealth`))) _aswb_aihealth_bar))

(fn `UserConstructionScript`)