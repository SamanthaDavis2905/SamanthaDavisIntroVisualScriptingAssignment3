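; BP_PitTrigger is a pit hazard that damages the player and teleports them out.
; When the player character overlaps its Box, it casts to BP_ThirdPersonCharacter, applies PitDamage and updates the health bar.
; It then teleports the character to DestLocation with a fixed rotation and stops movement immediately, clearing the fall velocity.
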(event `self.Box.OnComponentBeginOverlap`
  (params (OverlappedComponent :type "PrimitiveComponent Object Reference") (OtherActor :type "Actor Object Reference") (OtherComp :type "PrimitiveComponent Object Reference") (OtherBodyIndex :type Integer) (bFromSweep :type Boolean) (SweepResult :type "HitResult Structure (by ref)"))
  (bind _returnvalue (`GameplayStatics.GetPlayerCharacter` 0))
  (if (== OtherActor _returnvalue)
    (bind _asbp_third_person_character (cast `/Game/ThirdPerson/Blueprints/BP_ThirdPersonCharacter` _returnvalue))
    (`/Game/ThirdPerson/Blueprints/BP_ThirdPersonCharacter.PlayerTakeDamage` _asbp_third_person_character (`self.PitDamage`))
    (`/Game/ThirdPerson/Blueprints/BP_ThirdPersonCharacter.UpdatePlayerHealthbar` _asbp_third_person_character)
    (`self.K2_TeleportTo` _asbp_third_person_character (`self.Dest Location`) (struct :`Yaw` 180.0))
    (`MovementComponent.StopMovementImmediately` (`Character.CharacterMovement` _asbp_third_person_character))))

(fn `UserConstructionScript`)